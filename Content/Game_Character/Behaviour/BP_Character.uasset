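; Networked player character for what appears to be a racing runner, with automatic forward movement, slide, dash and finish-place icon.
; Authority Tick multicasts attribute-based walk speed, turning toward DesiredForwardVector, movement and icon updates, while remotes request movement via server RPC.
; Slide shrinks the capsule's Z scale; Dash overrides velocity, temporarily removing gravity or friction.
; Also handles camera zoom, side-view camera, in-game menu and a test montage key.
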(event Custom|Multicast_PlayMontage
  ;[1 1 1] Testing
  (CallFunction|PlayMontageonMesh))

(event Custom|MulticastUpdateSpeedFromAttribute
  ;[1 1 1] Multicast Events
  ;;[1 1 1] UpdateSpeedFromAttribute
  (CallFunction|ChangeWalkSpeedBasedonAttribute))

(event Custom|MulticastStartSlide
  (bind _originalecapsulerelscale (Variables|Default|GetOriginaleCapsuleRelScale))
  (bind (_x _y) (Math|Vector|BreakVector _originalecapsulerelscale))
  ;[1 1 1] Testing Slide
  (Variables|Default|SetbSlide true)
  (Transformation|SetRelativeScale3D (Variables|Default|GetCapsuleComponent) (Math|Vector|MakeVector _x _y 0.8)))

(event Custom|MulticastStopSlide
  ;[1 1 1] Testing Slide
  (Variables|Default|SetbSlide false)
  (Transformation|SetRelativeScale3D (Variables|Default|GetCapsuleComponent) (Variables|Default|GetOriginaleCapsuleRelScale)))

(event Custom|ServerStartSlide
  ;[1 1 1] Testing Slide
  (CallFunction|MulticastStartSlide))

(event Custom|ServerMoveForward
  ;[1 1 1] Multicast Events
  ;;[1 1 1] Add Forward Movement
  (CallFunction|MulticastMoveForward))

(event Custom|MulticastUpdateIcon
  ;[1 1 1] Multicast Events
  ;;[1 1 1] UpdateIcon
  (CallFunction|UpdateIcon))

(event Custom|Dash
  (params (DashSpeed :type Float%20%28single-precision%29) (DashDuration :type Float%20%28single-precision%29) (Sound :type Sound%20Base%20Object%20Reference))
  (bind _charactermovement (Variables|Character|GetCharacterMovement))
  (bind _charactermovement_2 (Variables|Character|GetCharacterMovement))
  (bind _desiredforwardvector (Variables|Default|GetDesiredForwardVector))
  (bind _charactermovement_3 (Variables|Character|GetCharacterMovement))
  (bind _returnvalue (* _desiredforwardvector DashSpeed))
  ;[1 1 1] Dash Ability
  (if (not (Class|NavMovementComponent|IsFlying _charactermovement_3))
    (CallFunction|SafeSetIsDashing true)
    (Audio|PlaySoundatLocation Sound (Transformation|GetActorLocation) "0, 0, 0" 1.0 1.0 0.0 0 0 0)
    (if (AI|Components|NavMovement|IsFalling _charactermovement_3)
      (Variables|/Script/Engine.MovementComponent|SetVelocity _charactermovement_2 _returnvalue)
      (Variables|/Script/Engine.CharacterMovementComponent|SetGravityScale _charactermovement_2 0.0)
      (Utilities|FlowControl|Delay DashDuration)
      (Variables|/Script/Engine.CharacterMovementComponent|SetGravityScale _charactermovement_2 1.0)
      (else
        (Variables|/Script/Engine.MovementComponent|SetVelocity _charactermovement _returnvalue)
        (Variables|/Script/Engine.CharacterMovementComponent|SetGroundFriction _charactermovement 0.0)
        (Variables|/Script/Engine.CharacterMovementComponent|SetBrakingDecelerationWalking _charactermovement 0.0)
        (Utilities|FlowControl|Delay DashDuration)
        (Variables|/Script/Engine.CharacterMovementComponent|SetBrakingDecelerationWalking _charactermovement (Variables|Default|GetBaseWalkBrakingDeceleration))
        (Variables|/Script/Engine.CharacterMovementComponent|SetGroundFriction _charactermovement 8.0)))
    (Variables|/Script/Engine.MovementComponent|SetVelocity (Variables|Character|GetCharacterMovement) (Variables|Default|GetBaseVelocity))
    (Utilities|FlowControl|Delay 0.1)
    (CallFunction|SafeSetIsDashing false)))

(event Custom|Server_PlayerMontage
  ;[1 1 1] Testing
  (CallFunction|MulticastPlayMontage))

(event Custom|MulticastTurn
  (bind _returnvalue (Pawn|GetController))
  (bind _desiredforwardvector (Variables|Default|GetDesiredForwardVector))
  (bind _returnvalue_2 (Math|Conversions|RotationFromXVector _desiredforwardvector))
  ;[1 1 1] Turning when overlap with Turnzone
  (if (Variables|Default|GetCanTurn)
    (Utilities|IsValid _returnvalue
      (:Is%20Valid
        (if (Utilities|Enum|NotEqual(Enum) _returnvalue_2 (Pawn|GetControlRotation :!class /Script/Engine.Pawn) 0.005)
          (Pawn|SetControlRotation _returnvalue (Math|Interpolation|RInterpTo (Transformation|GetActorRotation) _returnvalue_2 (Utilities|Time|GetWorldDeltaSeconds) 1.0))
          (else
            (Networking|SwitchHasAuthority
              (:Authority
                (Variables|Default|SetCanTurn false)))))))))

(event Custom|MulticastMoveForward
  ;[1 1 1] Multicast Events
  ;;[1 1 1] Add Forward Movement
  (CallFunction|AddAutomaticForwardMovement))

(event Custom|ServerStopSlide
  ;[1 1 1] Testing Slide
  (CallFunction|MulticastStopSlide))

(event EventBeginPlay
  (bind _charactermovement (Variables|Character|GetCharacterMovement))
  ;[1 1 1] Initialize variables on beginplay
  (Variables|Default|SetOriginaleCapsuleRelScale (Variables|/Script/Engine.SceneComponent|GetRelativeScale3D (Variables|Default|GetCapsuleComponent)))
  (Variables|Default|SetDesiredForwardVector "1.000000, 0, 0")
  (Variables|Default|SetBaseVelocity (Variables|/Script/Engine.MovementComponent|GetVelocity _charactermovement))
  (Variables|Default|SetBaseWalkBrakingDeceleration (Variables|/Script/Engine.CharacterMovementComponent|GetBrakingDecelerationWalking _charactermovement))
  (CallFunction|ChangeCameraView))

(event EventTick
  (params (DeltaSeconds :type Float%20%28single-precision%29))
  ;[1 1 1] Setup Movement
  (Networking|SwitchHasAuthority
    (:Authority
      (CallFunction|MulticastUpdateSpeedfromAttribute)
      (CallFunction|MulticastTurn)
      (CallFunction|MulticastMoveForward)
      (CallFunction|MulticastUpdateIcon))
    (:Remote
      (CallFunction|ServerMoveForward))))

(event Input|ActionEvents|InputActionProgInGameMenu
  (params (Key :type Key%20Structure))
  ;[1 1 1] Handle InGameMenu
  (:Released
    (bind _asrhgame_instance (Utilities|Casting|CastToRHGameInstance (Game|GetGameInstance)))
    (Utilities|FlowControl|FlipFlop
      (:A
        (Class|RHGameInstance|LoadMenuWidget _asrhgame_instance "/Game/UI/Menu/WBP_InGameMenu.WBP_InGameMenu_C"))
      (:B
        (Class|RHGameInstance|ExitMenu _asrhgame_instance)))))

(event Input|ActionEvents|InputActionCrouch
  (params (Key :type Key%20Structure))
  ;[1 1 1] Testing
  (:Pressed
    (Networking|SwitchHasAuthority
      (:Authority
        (CallFunction|MulticastStartSlide))
      (:Remote
        (CallFunction|ServerStartSlide))))
  (:Released
    (Networking|SwitchHasAuthority
      (:Authority
        (CallFunction|MulticastStopSlide))
      (:Remote
        (CallFunction|ServerStopSlide)))))

(event Input|KeyboardEvents|M
  (params (Key :type Key%20Structure))
  ;[1 1 1] Testing
  (:Pressed
    (Networking|SwitchHasAuthority
      (:Authority
        (CallFunction|MulticastPlayMontage))
      (:Remote
        (CallFunction|ServerPlayerMontage)))))

(event Input|MouseEvents|MouseWheelDown
  (params (Key :type Key%20Structure))
  (bind _cameraboom (Variables|Default|GetCameraBoom))
  ;[1 1 1] Camera Zoom Control
  (:Pressed
    (Variables|/Script/Engine.SpringArmComponent|SetTargetArmLength _cameraboom (Math|Float|Clamp(Float) (+ (Variables|/Script/Engine.SpringArmComponent|GetTargetArmLength _cameraboom) 25.0) 3e+02 6e+02))))

(event Input|MouseEvents|MouseWheelUp
  (params (Key :type Key%20Structure))
  (bind _cameraboom (Variables|Default|GetCameraBoom))
  ;[1 1 1] Camera Zoom Control
  (:Pressed
    (Variables|/Script/Engine.SpringArmComponent|SetTargetArmLength _cameraboom (Math|Float|Clamp(Float) (- (Variables|/Script/Engine.SpringArmComponent|GetTargetArmLength _cameraboom) 25.0) 3e+02 6e+02))))

(fn ConstructionScript)

(fn PlayMontageonMesh
  (Animation|Montage|MontagePlay (Components|SkeletalMesh|GetAnimInstance (Variables|Character|GetMesh)) "/Game/Game_Character/Animations/Montage/AM_ShockWave_Attack.AM_ShockWave_Attack" 1.0 "MontageLength" 0.0 true))

(fn ChangeCameraView
  (if (Variables|Default|GetbInSideViewMode)
    (Components|Activation|SetActive (Variables|Default|GetCameraRear) true false)
    (Components|Activation|SetActive (Variables|Default|GetFollowCamera) false false)))

(fn AddAutomaticForwardMovement
  (if (Variables|Default|GetbInRunMode)
    (Pawn|Input|AddMovementInput (Variables|Default|GetDesiredForwardVector) 1.0 false)))

(fn GetMoveForwardVal
  (return (Variables|Default|GetMoveForwardValue)))

(fn GetMoveRightVal
  (return (Variables|Default|GetMoveRightValue)))

(fn SetStats
  (params (StatsStruct :type Struct%20Stats%20Structure))
  (Variables|/Script/Engine.CharacterMovementComponent|SetMaxWalkSpeed (Variables|Character|GetCharacterMovement) (.Speed (Utilities|Struct|BreakStruct_Stats StatsStruct))))

(fn UpdateIcon
  (bind _asrhplayer_state (Utilities|Casting|CastToRHPlayerState (Variables|Default|GetPlayerState)))
  (if (< (Class|RHPlayerState|GetFinalPosition _asrhplayer_state) 100)
    (switch int (Math|Integer|%(Integer) (+ (Class|RHPlayerState|GetFinalPosition _asrhplayer_state) 1) 10)
      (:Default
        (LocalVariables|SetNumberPostfix "th" :!label _label))
      (:0
        (goto _label))
      (:1
        (LocalVariables|SetNumberPostfix "st"))
      (:2
        (LocalVariables|SetNumberPostfix "nd"))
      (:3
        (LocalVariables|SetNumberPostfix "rd")))
    (LocalVariables|SetFinalString (Utilities|String|Append (Utilities|String|ToString(Integer) (+ (Class|RHPlayerState|GetFinalPosition _asrhplayer_state) 1)) (LocalVariables|GetNumberPostfix) " Place"))
    (bind _aswbp_player_finish_icon (Utilities|Casting|CastToWBP_PLayerFinishIcon (UserInterface|GetUserWidgetObject (Variables|Default|GetIcon))))
    (Rendering|Components|TextRender|SetText (Variables|/Game/UI/WBP_PLayerFinishIcon.WBP_PLayerFinishIcon_C|GetTextBlock_Finish _aswbp_player_finish_icon) (Utilities|Text|ToText(String) (LocalVariables|GetFinalString)))))

(fn ChangeWalkSpeedBasedonAttribute
  (bind _returnvalue (Class|ProjectRHCharacter|GetMoveSpeed))
  (bind _basewalkspeed (Variables|Default|GetBaseWalkSpeed))
  (bind _returnvalue_2 (* _returnvalue _basewalkspeed))
  (if (!= _returnvalue_2 (Variables|Default|GetOldWalkSpeed))
    (Variables|Default|SetOldWalkSpeed _returnvalue_2)
    (Variables|/Script/Engine.CharacterMovementComponent|SetMaxWalkSpeed (Variables|Character|GetCharacterMovement) _returnvalue_2)))

(fn SafeSetIsDashing
  (params (IsDashing :type Boolean))
  (Networking|SwitchHasAuthority
    (:Authority
      (Variables|Default|SetIsDashing IsDashing))))