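; Electric zap power-up that slows the nearest character in the owner's attack zone and links to them with an electric arc.
; On activation a timeline scales the target's walk speed, then destroys the actor when finished.
; In parallel, the owner plays a hand montage, then spawns a beam that re-targets the victim on a delay loop until deactivated.
; Without a target, it clears the owner's power-up activated flag.
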(event EventBeginPlay)

(event Collision|EventActorBeginOverlap
  (params (OtherActor :type Actor%20Object%20Reference)))

(event EventTick
  (params (DeltaSeconds :type Float%20%28single-precision%29)))

(event EventOnActivate
  ;[1 1 1] Processing Activation
  (bind _asproject_rhcharacter (CallFunction|GetNearestOverlapCharacter))
  (Utilities|IsValid _asproject_rhcharacter
    (:Is%20Valid
      (Variables|Default|SetDamagedChar _asproject_rhcharacter)
      (Utilities|FlowControl|Sequence
        (:then_0
          (Variables|Default|SetOriginalSpeed (Variables|/Script/Engine.CharacterMovementComponent|GetMaxWalkSpeed (Variables|/Script/Engine.Character|GetCharacterMovement (Variables|Default|GetDamagedChar))))
          (bind _speedfactor (Timeline|Timeline_DecreaseSpeed Play)
            (:Update
              (Variables|/Script/Engine.CharacterMovementComponent|SetMaxWalkSpeed (Variables|/Script/Engine.Character|GetCharacterMovement (Variables|Default|GetDamagedChar)) (* _speedfactor (Variables|Default|GetOriginalSpeed))))
            (:Finished
              (Actor|DestroyActor))))
        (:then_1
          (CallFunction|PlayHandAnimation)
          (Utilities|FlowControl|Delay 0.5)
          (bind _returnvalue (Effects|SpawnEmitterAttached "/Game/Effect/ParticleSystems/P_electricity_arc.P_electricity_arc" (Variables|/Script/Engine.Character|GetMesh (Variables|Default|GetOwningCharacter)) (Variables|Default|GetDamageSourcePoint) "0, 0, 0" "0, 0, 0" "1.000000,1.000000,1.000000" "SnapToTargetIncludingScale"))
          (Variables|Default|SetPowerUpPartSysComp _returnvalue)
          (CallFunction|SetNewBeamTarget :!label _label)
          (Utilities|FlowControl|Sequence
            (:then_0
              (Utilities|FlowControl|Delay (Variables|Default|GetZapDuration))
              (CallFunction|DeactivatePowerUpParticleSystem))
            (:then_1
              (Utilities|FlowControl|Delay 0.1)
              (goto _label))))))
    (:Is%20Not%20Valid
      (CallFunction|ReactivateAcquiringAbility))))

(fn ConstructionScript)

(fn PlayHandAnimation
  (Animation|Montage|MontagePlay (Components|SkeletalMesh|GetAnimInstance (Variables|/Script/Engine.Character|GetMesh (Variables|Default|GetOwningCharacter))) "/Game/Game_Character/Animations/Montage/AM_Magic_Heal.AM_Magic_Heal" 1.0 "MontageLength" 0.0 true))

(fn DeactivatePowerUpParticleSystem
  (bind _poweruppartsyscomp (Variables|Default|GetPowerUpPartSysComp))
  (Utilities|IsValid _poweruppartsyscomp
    (:Is%20Valid
      (Components|Activation|Deactivate _poweruppartsyscomp))))

(fn SetNewBeamTarget
  (bind _poweruppartsyscomp (Variables|Default|GetPowerUpPartSysComp))
  (Utilities|IsValid _poweruppartsyscomp
    (:Is%20Valid
      (Class|ParticleSystemComponent|SetBeamTargetPoint _poweruppartsyscomp 0 (Transformation|GetSocketLocation (Variables|/Script/Engine.Character|GetMesh (Variables|Default|GetDamagedChar)) (Variables|Default|GetDamagePoint))))))

(fn GetNearestOverlapCharacter
  (bind _owningcharacter (Variables|Default|GetOwningCharacter))
  (bind _asbp_character (Utilities|Casting|CastToBP_Character (Variables|Default|GetOwningCharacter))
    (:then
      (if (> (Utilities|Array|Length (Collision|GetOverlappingActors (Class|ProjectRHCharacter|GetAttackZone _asbp_character) "/Script/ProjectRH.ProjectRHCharacter" :!class /Script/Engine.PrimitiveComponent)) 0)
        (LocalVariables|SetNearestCharacter (Utilities|Array|Get(acopy) (Collision|GetOverlappingActors (Class|ProjectRHCharacter|GetAttackZone _asbp_character) "/Script/ProjectRH.ProjectRHCharacter" :!class /Script/Engine.PrimitiveComponent)))
        (for _array_element (Collision|GetOverlappingActors (Class|ProjectRHCharacter|GetAttackZone _asbp_character) "/Script/ProjectRH.ProjectRHCharacter" :!class /Script/Engine.PrimitiveComponent)
          (if (< (Transformation|GetDistanceTo _array_element _owningcharacter) (Transformation|GetDistanceTo _owningcharacter (LocalVariables|GetNearestCharacter)))
            (LocalVariables|SetNearestCharacter _array_element)))
        (bind _asproject_rhcharacter (Utilities|Casting|CastToProjectRHCharacter (LocalVariables|GetNearestCharacter))
          (:then
            (return _asproject_rhcharacter))
          (:CastFailed
            (return 0)))
        (else
          (return 0))))
    (:CastFailed
      (return 0))))

(fn ReactivateAcquiringAbility
  (bind _owningcharacter (Variables|Default|GetOwningCharacter))
  (Utilities|IsValid _owningcharacter
    (:Is%20Valid
      (Class|ProjectRHCharacter|SetPowerUpActivated _owningcharacter false))))