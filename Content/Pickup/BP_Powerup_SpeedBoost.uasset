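; Speed boost powerup that temporarily raises the walk speed of the character who activates it.
; Activate stores the player character, multiplies its MaxWalkSpeed by BoostFactor, waits BoostDuration, then applies the inverse factor and destroys itself.
; The multiply-and-divide approach scales the current speed rather than restoring a saved value.
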(event EventActivate
  (params (PlayerChar :type Project%20RH%20Character%20Object%20Reference))
  ;[1 1 1] Activate Speed Boost
  (Utilities|IsValid PlayerChar
    (:Is%20Valid
      (Variables|Default|SetPlayerCharacter PlayerChar)
      (CallFunction|SetCharacterWalkSpeed (Variables|Default|GetBoostFactor))
      (Utilities|FlowControl|Delay (Variables|Default|GetBoostDuration))
      (CallFunction|SetCharacterWalkSpeed (/ 1.0 (Variables|Default|GetBoostFactor)))
      (Actor|DestroyActor))))

(fn ConstructionScript)

(fn SetCharacterWalkSpeed
  (params (Factor :type Float%20%28single-precision%29))
  (bind _playercharacter (Variables|Default|GetPlayerCharacter))
  (bind _charactermovement (Variables|/Script/Engine.Character|GetCharacterMovement _playercharacter))
  (Variables|/Script/Engine.CharacterMovementComponent|SetMaxWalkSpeed _charactermovement (* (Variables|/Script/Engine.CharacterMovementComponent|GetMaxWalkSpeed _charactermovement) Factor)))