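; Flight powerup that puts the owning character into Flying movement mode for a limited time.
; On activation it disables orient-rotation-to-movement and plays a timeline that serves as the duration timer.
; When the timeline finishes it restores Walking, re-enables rotation through MulticastResetOrientRotationToMovement and destroys itself.
; SpawnSpeedBoostAttached, which attaches a particle effect to the head socket, keeps speed-boost naming, as does the timeline.
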(event Custom|MulticastResetOrientRotationToMovement
  ;[1 1 1] Activate Speed Boost
  (Variables|/Script/Engine.CharacterMovementComponent|SetbOrientRotationToMovement (Variables|/Script/Engine.Character|GetCharacterMovement (Variables|Default|GetOwningCharacter)) true))

(event EventOnActivate
  (bind _owningcharacter (Variables|Default|GetOwningCharacter))
  (bind _charactermovement (Variables|/Script/Engine.Character|GetCharacterMovement _owningcharacter))
  ;[1 1 1] Activate Speed Boost
  (Pawn|Components|CharacterMovement|SetMovementMode _charactermovement "MOVE_Flying" 0)
  (Variables|/Script/Engine.CharacterMovementComponent|SetbOrientRotationToMovement _charactermovement false)
  (Timeline|Timeline_SpeedBoost Play
    (:Finished
      (Pawn|Components|CharacterMovement|SetMovementMode _charactermovement "MOVE_Walking" 0)
      (CallFunction|MulticastResetOrientRotationtoMovement)
      (Actor|DestroyActor))))

(fn ConstructionScript)

(fn SpawnSpeedBoostAttached
  (bind _returnvalue (Effects|SpawnEmitterAttached "/Engine/Tutorial/SubEditors/TutorialAssets/TutorialParticleSystem.TutorialParticleSystem" (Variables|/Script/Engine.Character|GetMesh (Variables|Default|GetOwningCharacter)) "HeadSocket" "0, 0, 0" "0, 0, 0" "1.000000,1.000000,1.000000" "SnapToTargetIncludingScale"))
  (bind _output_get (Variables|Default|SetParSysComp _returnvalue))
  (return _output_get))