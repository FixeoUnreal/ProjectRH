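; BP_Obstacle is a terrain prop with an unfinished slow-down effect for overlapping characters.
; Its overlap event is empty, and the effect logic is disconnected, so it never runs.
; That logic would scale a BP_Character's walk speed through a timeline, spawn a particle effect and destroy the obstacle when finished.
; OriginalSpeed is set to zero there rather than read from the movement component.
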(event Custom|OnBeginOverlap_1
  (params (OverlappingCharacter :type Project%20RH%20Character%20Object%20Reference))
  ;[1 1 1] Slow-Down-Effect
)

(event EventBeginPlay)

(event Collision|EventActorBeginOverlap
  (params (OtherActor :type Actor%20Object%20Reference)))

(event EventTick
  (params (DeltaSeconds :type Float%20%28single-precision%29)))

(fn ConstructionScript)