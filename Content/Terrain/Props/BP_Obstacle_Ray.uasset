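; BP_Obstacle_Ray is a terrain obstacle prop that forms a beam between two meshes, with a collision box spanning the gap.
; On BeginPlay it sets the particle beam's target to MeshComp's BeamSource socket and makes the effect visible.
; It then centers the box between both meshes' BeamSource sockets, aligns its Y axis along the beam and sets that half-extent to half the distance.
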(event EventBeginPlay
  (bind _particlesystem (Variables|Default|GetParticleSystem))
  (bind _meshcomp (Variables|Default|GetMeshComp))
  (bind _staticmesh (Variables|Default|GetStaticMesh))
  (bind _boxcollision (Variables|Default|GetBoxCollision))
  (bind _returnvalue (Transformation|GetSocketLocation _staticmesh "BeamSource"))
  (bind _returnvalue_2 (Transformation|GetSocketLocation _meshcomp "BeamSource"))
  (bind _boxextent (Variables|/Script/Engine.BoxComponent|GetBoxExtent _boxcollision))
  (bind (_x _y _z) (Math|Vector|BreakVector _boxextent))
  (bind _returnvalue_3 (- _returnvalue _returnvalue_2))
  (Class|ParticleSystemComponent|SetBeamTargetPoint _particlesystem 0 _returnvalue_2)
  (Rendering|SetVisibility _particlesystem true true)
  (Transformation|SetWorldRotation _boxcollision (Math|Rotator|MakeRotfromY _returnvalue_3) false false)
  (Components|Box|SetBoxExtent _boxcollision (Math|Vector|MakeVector _x (/ (Math|Vector|VectorLength _returnvalue_3) 2.0) _z) true)
  (Transformation|SetWorldLocation _boxcollision (+ _returnvalue_2 (/ _returnvalue_3 2.0)) false false))

(fn ConstructionScript)