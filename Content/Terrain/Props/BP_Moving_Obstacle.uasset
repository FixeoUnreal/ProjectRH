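; Moving obstacle actor that shuttles back and forth in a straight line between its spawn point and a Destination component's world position.
; Both endpoints are cached on BeginPlay, then Tick moves it at a constant speed while Move is enabled, without sweeping.
; Once its distance from the start exceeds the path length, it swaps the endpoints and flips its forward vector to face the return direction.
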(event Custom|MoveBackAndForth
  (params (DeltaSeconds :type Float%20%28single-precision%29))
  ;[1 1 1] Move actor back and forth based on destination and speed in cm/s
  (if (Variables|Default|GetbMove)
    (if (CallFunction|IsatDestination)
      (CallFunction|SwapLocationandRotation)
      (else
        (Transformation|SetActorLocation (+ (CallFunction|GetVelocityPerFrame DeltaSeconds) (Transformation|GetActorLocation)) false false)))))

(event EventBeginPlay
  (Variables|Default|SetStartLocation (Transformation|GetActorLocation))
  (Variables|Default|SetTargetLocation (Transformation|GetWorldLocation (Variables|Default|GetDestination))))

(event EventTick
  (params (DeltaSeconds :type Float%20%28single-precision%29))
  (CallFunction|MoveBackandForth DeltaSeconds))

(fn ConstructionScript)

(fn GetVelocityPerFrame
  (params (DeltaSeconds :type Float%20%28single-precision%29))
  (return (* (* (Math|Vector|Normalize (- (Variables|Default|GetTargetLocation) (Variables|Default|GetStartLocation))) (Math|Float|Absolute(Float) (Variables|Default|GetSpeed))) DeltaSeconds)))

(fn IsatDestination
  (bind _startlocation (Variables|Default|GetStartLocation))
  (return (> (Math|Vector|VectorLength (- (Transformation|GetActorLocation) _startlocation)) (Math|Vector|VectorLength (- _startlocation (Variables|Default|GetTargetLocation))))))

(fn SwapLocationandRotation
  (LocalVariables|SetTempLocation (Variables|Default|GetTargetLocation))
  (Variables|Default|SetTargetLocation (Variables|Default|GetStartLocation))
  (Variables|Default|SetStartLocation (LocalVariables|GetTempLocation))
  (Transformation|SetActorRotation (Math|Conversions|RotationFromXVector (* (Math|Vector|GetForwardVector (Transformation|GetActorRotation)) -1))))