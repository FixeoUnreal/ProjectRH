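; BP_Turn_Base is a terrain actor, named as a base, that marks a zone where characters are allowed to turn.
; On the server only, a BP_Character entering TurnBox gets CanTurn set and receives TurnDirection's normalized forward vector as its DesiredForwardVector.
; Leaving the box clears CanTurn; the turn itself is not performed in this Blueprint.
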(event OnComponentBeginOverlap(TurnBox)
  (params (OverlappedComponent :type Primitive%20Component%20Object%20Reference) (OtherActor :type Actor%20Object%20Reference) (OtherComp :type Primitive%20Component%20Object%20Reference) (OtherBodyIndex :type Integer) (bFromSweep :type Boolean) (SweepResult :type Hit%20Result%20Structure%20%28by%20ref%29))
  ;[1 1 1] Handle Turning
  (Networking|SwitchHasAuthority
    (:Authority
      (bind _asbp_character (Utilities|Casting|CastToBP_Character OtherActor))
      (Variables|/Game/Game_Character/Behaviour/BP_Character.BP_Character_C|SetCanTurn _asbp_character true)
      (Variables|/Script/ProjectRH.ProjectRHCharacter|SetDesiredForwardVector _asbp_character (Math|Vector|Normalize (Math|Vector|GetForwardVector (Variables|Default|GetTurnDirection)))))))

(event OnComponentEndOverlap(TurnBox)
  (params (OverlappedComponent :type Primitive%20Component%20Object%20Reference) (OtherActor :type Actor%20Object%20Reference) (OtherComp :type Primitive%20Component%20Object%20Reference) (OtherBodyIndex :type Integer))
  ;[1 1 1] Handle Turning
  (Networking|SwitchHasAuthority
    (:Authority
      (bind _asbp_character (Utilities|Casting|CastToBP_Character OtherActor))
      (Variables|/Game/Game_Character/Behaviour/BP_Character.BP_Character_C|SetCanTurn _asbp_character false))))

(event EventBeginPlay)

(event Collision|EventActorBeginOverlap
  (params (OtherActor :type Actor%20Object%20Reference)))

(event EventTick
  (params (DeltaSeconds :type Float%20%28single-precision%29)))

(fn ConstructionScript)