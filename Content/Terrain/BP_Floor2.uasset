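; BP_Floor2 is a floor tile actor for an endlessly spawning path, chaining copies of itself as the player advances.
; When a ProjectRHCharacter overlaps SpawningBox, it spawns another BP_Floor2 at the ArrowComp's world transform.
; When the character overlaps DestroyingBox, the tile destroys itself.
; GetAttachLocation also exposes that arrow transform as the attach point for the next piece.
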(event OnComponentBeginOverlap(SpawningBox)
  (params (OverlappedComponent :type Primitive%20Component%20Object%20Reference) (OtherActor :type Actor%20Object%20Reference) (OtherComp :type Primitive%20Component%20Object%20Reference) (OtherBodyIndex :type Integer) (bFromSweep :type Boolean) (SweepResult :type Hit%20Result%20Structure%20%28by%20ref%29))
  (Utilities|Casting|CastToProjectRHCharacter OtherActor)
  (Game|SpawnActorfromClass "BP_Floor2_C" (Transformation|GetWorldTransform (Variables|Default|GetArrowComp)) "Undefined" 0 0))

(event OnComponentBeginOverlap(DestroyingBox)
  (params (OverlappedComponent :type Primitive%20Component%20Object%20Reference) (OtherActor :type Actor%20Object%20Reference) (OtherComp :type Primitive%20Component%20Object%20Reference) (OtherBodyIndex :type Integer) (bFromSweep :type Boolean) (SweepResult :type Hit%20Result%20Structure%20%28by%20ref%29))
  (Utilities|Casting|CastToProjectRHCharacter OtherActor)
  (Actor|DestroyActor))

(event EventBeginPlay)

(event Collision|EventActorBeginOverlap
  (params (OtherActor :type Actor%20Object%20Reference)))

(event EventTick
  (params (DeltaSeconds :type Float%20%28single-precision%29)))

(fn ConstructionScript)

(fn GetAttachLocation
  (return (Transformation|GetWorldTransform (Variables|Default|GetArrowComp))))