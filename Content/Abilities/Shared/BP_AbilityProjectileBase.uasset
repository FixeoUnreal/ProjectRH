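; Base ability projectile Blueprint that applies gameplay effects to actors it overlaps in flight.
; On overlap it records each actor in HitActors so each is handled only once, and skips applying effects to its instigator.
; For other actors it adds them as targets to its EffectContainerSpec, generated when the projectile spawns, and applies that spec as an external effect container.
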(event Collision|EventActorBeginOverlap
  (params (OtherActor :type Actor%20Object%20Reference))
  (bind _hitactors (Variables|Default|GetHitActors))
  (if (not (Utilities|Array|ContainsItem _hitactors OtherActor)) ; Make sure we only hit each actor once
    (Utilities|Array|Add _hitactors OtherActor)
    (if (!= OtherActor (Game|GetInstigator))
      (bind _returnvalue (Class|RHBlueprintFunctionLibrary|AddTargetstoEffectContainerSpec (Variables|Default|GetEffectContainerSpec) 0 (Utilities|Array|MakeArray OtherActor))) ; Modify the container spec to target the actors we overlapped with
      (Class|RHBlueprintFunctionLibrary|ApplyExternalEffectContainerSpec _returnvalue) ; Applies effect, uses information generated when projectile is spawned
    )))

(fn ConstructionScript)