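; Gameplay ability that performs a dash on the owning character.
; On activation it casts the avatar actor to BP_Character and calls its Dash function with the ability's speed, duration and sound settings.
; It ends immediately after that call, or cancels when the avatar is invalid or not a BP_Character.
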(event Ability|EventActivateAbility
  (bind _returnvalue (Ability|GetAvatarActorfromActorInfo))
  ;[1 1 1] Use Dash with specific settings
  (|CallParentFunction)
  (Utilities|IsValid _returnvalue
    (:Is%20Valid
      (bind _asbp_character (Utilities|Casting|CastToBP_Character _returnvalue)
        (:then
          (Default|Dash _asbp_character (Variables|Default|GetDashSpeed) (Variables|Default|GetDashDuration) (Variables|Default|GetSound))
          (Ability|EndAbility))
        (:CastFailed
          (Ability|CancelAbility :!label _label))))
    (:Is%20Not%20Valid
      (goto _label))))

(event Ability|EventOnEndAbility
  (params (bWasCancelled :type Boolean))
  (|CallParentFunction bWasCancelled) ; This node is disabled and will not be called.\nDrag off pins to build functionality.
)